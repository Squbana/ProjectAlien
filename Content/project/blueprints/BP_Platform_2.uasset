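; BP_Platform_2 is an elevator platform that moves vertically once the third-person character overlaps its Box trigger.
; BeginPlay caches the actor's starting Z and adds Distance to get the final height.
; The overlap plays a Timeline from the start, lerping Z between those heights while keeping X and Y, with no return logic.
; A disconnected sine-wave oscillation variant remains in the graph but never runs.
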(event OnComponentBeginOverlap(Box)
  (params (OverlappedComponent :type Primitive%20Component%20Object%20Reference) (OtherActor :type Actor%20Object%20Reference) (OtherComp :type Primitive%20Component%20Object%20Reference) (OtherBodyIndex :type Integer) (bFromSweep :type Boolean) (SweepResult :type Hit%20Result%20Structure%20%28by%20ref%29))
  (Utilities|Casting|CastToBP_ThirdPersonCharacter OtherActor)
  (CallFunction|ElevatorMoveup))

(event Custom|ElevatorMoveup
  (bind _returnvalue (Transformation|GetActorLocation))
  ;[1 1 1] timeline
  (bind _newtrack_0 (Timeline|Timeline PlayFromStart)
    (:Update
      (Transformation|SetActorLocation (Math|Vector|MakeVector (.x _returnvalue) (.y _returnvalue) (Math|Float|Lerp (Variables|Default|GetStartLocation) (Variables|Default|GetFinalLocation) _newtrack_0)) false false))))

(event EventBeginPlay
  ;[1 1 1] pobieranie lokacji do lerp'a
  (bind _output_get (Variables|Default|SetStartLocation (.z (Transformation|GetActorLocation))))
  (Variables|Default|SetFinalLocation (+ _output_get (Variables|Default|GetDistance))))

(event Collision|EventActorBeginOverlap
  (params (OtherActor :type Actor%20Object%20Reference)))

(event EventTick
  (params (DeltaSeconds :type Float%20%28single-precision%29)))

(fn ConstructionScript)