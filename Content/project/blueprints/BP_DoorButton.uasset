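; BP_DoorButton is an interactable button meant to open the BP_Doors_OnButton door whose DoorOnButtonValue equals its ButtonValue.
; Interact searches all such doors and, on a match, plays the ButtonPress timeline to slide the Cylinder along Y.
; When the timeline finishes, a short delay precedes OpenButtonDoor and the loop break.
; The loop does not wait for the timeline, so the element opened then may differ from the match.
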(event EventInteract
  (params (Player :type Character%20Object%20Reference))
  (bind _outactors (Actor|GetAllActorsOfClass "/Game/project/blueprints/BP_Doors_OnButton.BP_Doors_OnButton_C"))
  (bind _array_element (Utilities|Array|ForEachLoopwithBreak _outactors :!label _label)
    (:LoopBody
      (if (== (Variables|/Game/project/blueprints/BP_Doors_OnButton.BP_Doors_OnButton_C|GetDoor_OnButton_Value _array_element) (Variables|Default|GetButtonValue))
        ;[1 1 1] PressButtonAnimation
        (bind _buttontrack (Timeline|ButtonPress Play)
          (:Update
            (Transformation|SetRelativeLocation (Variables|Default|GetCylinder) (Math|Vector|MakeVector 0.0 _buttontrack 0.0) false false))
          (:Finished
            (Utilities|FlowControl|Delay 0.2)
            (Default|OpenButtonDoor _array_element)
            (goto _label Break)))))))

(fn ConstructionScript)