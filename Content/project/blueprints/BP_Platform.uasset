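; BP_Platform is an elevator platform actor that moves vertically over a set Distance from its starting height.
; BeginPlay records the start and final Z, then calls ElevatorMove, which plays a timeline that lerps the actor's Z between them while keeping X and Y.
; An alternative sine-of-game-time oscillation is left disconnected, and Tick is empty.
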(event Custom|ElevatorMove
  (bind _returnvalue (Transformation|GetActorLocation))
  ;[1 1 1] timeline
  (bind _newtrack_0 (Timeline|Timeline PlayFromStart)
    (:Update
      (Transformation|SetActorLocation (Math|Vector|MakeVector (.x _returnvalue) (.y _returnvalue) (Math|Float|Lerp (Variables|Default|GetStartLocation) (Variables|Default|GetFinalLocation) _newtrack_0)) false false))))

(event EventBeginPlay
  ;[1 1 1] pobieranie lokacji do lerp'a
  (bind _output_get (Variables|Default|SetStartLocation (.z (Transformation|GetActorLocation))))
  (Variables|Default|SetFinalLocation (+ _output_get (Variables|Default|GetDistance)))
  (CallFunction|ElevatorMove))

(event Collision|EventActorBeginOverlap
  (params (OtherActor :type Actor%20Object%20Reference)))

(event EventTick
  (params (DeltaSeconds :type Float%20%28single-precision%29)))

(fn ConstructionScript)