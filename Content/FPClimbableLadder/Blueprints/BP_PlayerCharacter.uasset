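; First-person player character for the climbable ladder system, handling look, movement, jog speed, and jumping with jump and landing camera shakes.
; Move axes drive movement input and are also stored through update events.
; Jump either sends a leave message to the active parkour actor, or offers an enter message to every BP_ParkourActor in the level and then jumps.
; Number keys switch debug drawing on all ladders.
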(event Custom|UpdateMoveX
  (params (MoveX :type Float%20%28double-precision%29))
  ;[0 0 0] Movement Inputs / Tick Events
  (Variables|Default|SetMoveX MoveX))

(event Custom|UpdateMoveY
  (params (MoveY :type Float%20%28double-precision%29))
  ;[0 0 0] Movement Inputs / Tick Events
  (Variables|Default|SetMoveY MoveY))

(event Custom|JumpEvent
  ;[0 0 0] Parkour/Jump Inputs
  (Character|Jump)
  (Game|Feedback|ClientStartCameraShake (Game|GetPlayerController 0) "/Game/FPClimbableLadder/Blueprints/CS_Jump.CS_Jump_C" 1.0 "CameraLocal" "0, 0, 0"))

(event Custom|ParkourEvent
  ;[0 0 0] Parkour/Jump Inputs
  (if (Variables|Default|GetbParkour)
    (bind _parkouractor (Variables|Default|GetParkourActor)
      (:then
        (Class|BPIParkour|ParkourLeave(Message) _parkouractor self))
      (:else))
    (else
      (bind _outactors (Actor|GetAllActorsOfClass "/Game/FPClimbableLadder/Blueprints/BP_ParkourActor.BP_ParkourActor_C"))
      (for _array_element _outactors
        (Class|BPIParkour|ParkourEnter(Message) _array_element self))
      (CallFunction|JumpEvent))))

(event EventOnLanded
  (params (Hit :type Hit%20Result%20Structure%20%28by%20ref%29))
  ;[0 0 0] Land Camera Shake
  (Game|Feedback|ClientStartCameraShake (Game|GetPlayerController 0) "/Game/FPClimbableLadder/Blueprints/CS_Land.CS_Land_C" 1.0 "CameraLocal" "0, 0, 0"))

(event Input|ActionEvents|InputActionJog
  (params (Key :type Key%20Structure :default "None"))
  (bind _charactermovement (Variables|Character|GetCharacterMovement))
  ;[0 0 0] Jog Inputs
  (:Pressed
    (Variables|/Script/Engine.CharacterMovementComponent|SetMaxWalkSpeed _charactermovement 1e+03))
  (:Released
    (Variables|/Script/Engine.CharacterMovementComponent|SetMaxWalkSpeed _charactermovement 6e+02)))

(event Input|ActionEvents|InputActionJump
  (params (Key :type Key%20Structure :default "None"))
  ;[0 0 0] Parkour/Jump Inputs
  (:Pressed
    (CallFunction|ParkourEvent)))

(event Input|AxisEvents|InputAxisMoveX
  (params (AxisValue :type Float%20%28single-precision%29))
  ;[0 0 0] Movement Inputs / Tick Events
  (bind _output_get (Variables|Default|SetClientMoveX AxisValue))
  (Pawn|Input|AddMovementInput (Transformation|GetActorRightVector) _output_get false)
  (CallFunction|UpdateMoveX (Variables|Default|GetClientMoveX)))

(event Input|AxisEvents|InputAxisMoveY
  (params (AxisValue :type Float%20%28single-precision%29))
  ;[0 0 0] Movement Inputs / Tick Events
  (bind _output_get (Variables|Default|SetClientMoveY AxisValue))
  (Pawn|Input|AddMovementInput (Transformation|GetActorForwardVector) _output_get false)
  (CallFunction|UpdateMoveY (Variables|Default|GetClientMoveY)))

(event Input|AxisEvents|InputAxisViewX
  (params (AxisValue :type Float%20%28single-precision%29))
  ;[0 0 0] View Inputs
  (Pawn|Input|AddControllerYawInput AxisValue))

(event Input|AxisEvents|InputAxisViewY
  (params (AxisValue :type Float%20%28single-precision%29))
  ;[0 0 0] View Inputs
  (Pawn|Input|AddControllerPitchInput AxisValue))

(event Input|KeyboardEvents|1
  (params (Key :type Key%20Structure :default "None"))
  ;[0 0 0] Draw Debug
  (:Pressed
    (bind _outactors (Actor|GetAllActorsOfClass "/Game/FPClimbableLadder/Blueprints/BP_ClimbableLadder.BP_ClimbableLadder_C"))
    (for _array_element _outactors
      (Variables|/Game/FPClimbableLadder/Blueprints/BP_ClimbableLadder.BP_ClimbableLadder_C|SetDraw%20Debug _array_element "None"))
    (Development|PrintString "Draw Debug: None")))

(event Input|KeyboardEvents|2
  (params (Key :type Key%20Structure :default "None"))
  ;[0 0 0] Draw Debug
  (:Pressed
    (bind _outactors (Actor|GetAllActorsOfClass "/Game/FPClimbableLadder/Blueprints/BP_ClimbableLadder.BP_ClimbableLadder_C"))
    (for _array_element _outactors
      (Variables|/Game/FPClimbableLadder/Blueprints/BP_ClimbableLadder.BP_ClimbableLadder_C|SetDraw%20Debug _array_element "ForOneFrame"))
    (Development|PrintString "Draw Debug: For One Frame")))

(event Input|KeyboardEvents|3
  (params (Key :type Key%20Structure :default "None"))
  ;[0 0 0] Draw Debug
  (:Pressed
    (bind _outactors (Actor|GetAllActorsOfClass "/Game/FPClimbableLadder/Blueprints/BP_ClimbableLadder.BP_ClimbableLadder_C"))
    (for _array_element _outactors
      (Variables|/Game/FPClimbableLadder/Blueprints/BP_ClimbableLadder.BP_ClimbableLadder_C|SetDraw%20Debug _array_element "ForDuration"))
    (Development|PrintString "Draw Debug: For Duration")))

(fn ConstructionScript)