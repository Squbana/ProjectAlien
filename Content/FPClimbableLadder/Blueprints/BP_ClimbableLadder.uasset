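; First-person climbable ladder actor whose construction script builds stacked meshes, a spline and side/top trigger boxes from LadderHeight.
; Triggers show an input prompt tracking the spline; interface entry checks view angle, while falling into the side trigger auto-attaches.
; Climbing uses custom movement mode, with timer-driven movement along the spline and camera shakes.
; Players jump off by looking away, or climb over the top when sphere traces find a clear ledge.
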(event OnComponentBeginOverlap(SideCollision)
  (params (OverlappedComponent :type Primitive%20Component%20Object%20Reference) (OtherActor :type Actor%20Object%20Reference) (OtherComp :type Primitive%20Component%20Object%20Reference) (OtherBodyIndex :type Integer) (bFromSweep :type Boolean) (SweepResult :type Hit%20Result%20Structure%20%28by%20ref%29))
  ;[0 0 0] Trigger Events for the Side Collision
  (bind _asbp_first_person_character (Utilities|Casting|CastToBP_FirstPersonCharacter OtherActor))
  (bind _output_get (Variables|ClimbableLadder|SetPlayer%20Character _asbp_first_person_character))
  (if (AI|Components|NavMovement|IsFalling (Variables|/Script/Engine.Character|GetCharacterMovement _output_get)) ; If the character enter the trigger volume when falling,\nthen climb up the ladder automatically.
    (CallFunction|StartClimbing)
    (else
      (Rendering|SetVisibility (Variables|Default|GetWidget) true false))))

(event OnComponentEndOverlap(SideCollision)
  (params (OverlappedComponent :type Primitive%20Component%20Object%20Reference) (OtherActor :type Actor%20Object%20Reference) (OtherComp :type Primitive%20Component%20Object%20Reference) (OtherBodyIndex :type Integer))
  ;[0 0 0] Trigger Events for the Side Collision
  (Utilities|Casting|CastToBP_FirstPersonCharacter OtherActor)
  (Rendering|SetVisibility (Variables|Default|GetWidget) false false))

(event OnComponentBeginOverlap(TopCollision)
  (params (OverlappedComponent :type Primitive%20Component%20Object%20Reference) (OtherActor :type Actor%20Object%20Reference) (OtherComp :type Primitive%20Component%20Object%20Reference) (OtherBodyIndex :type Integer) (bFromSweep :type Boolean) (SweepResult :type Hit%20Result%20Structure%20%28by%20ref%29))
  ;[0 0 0] Trigger Events for the Top Collision
  (bind _asbp_first_person_character (Utilities|Casting|CastToBP_FirstPersonCharacter OtherActor))
  (Variables|ClimbableLadder|SetPlayer%20Character _asbp_first_person_character)
  (Rendering|SetVisibility (Variables|Default|GetWidget) true false))

(event OnComponentEndOverlap(TopCollision)
  (params (OverlappedComponent :type Primitive%20Component%20Object%20Reference) (OtherActor :type Actor%20Object%20Reference) (OtherComp :type Primitive%20Component%20Object%20Reference) (OtherBodyIndex :type Integer))
  ;[0 0 0] Trigger Events for the Top Collision
  (Utilities|Casting|CastToBP_FirstPersonCharacter OtherActor)
  (Rendering|SetVisibility (Variables|Default|GetWidget) false false))

(event Custom|Ladder%20Movement
  (bind _spline (Variables|Default|GetSpline))
  (bind _player_character (Variables|ClimbableLadder|GetPlayer%20Character))
  (bind _spline_2 (Variables|Default|GetSpline))
  (bind _player_character_2 (Variables|ClimbableLadder|GetPlayer%20Character))
  (bind _returnvalue (Spline|GetTransformatTime _spline_2 1.0 "World" false false))
  (bind _returnvalue_2 (Transformation|GetActorLocation _player_character_2))
  (bind _returnvalue_3 (Transformation|GetActorUpVector _player_character_2))
  (bind _capsulecomponent (Variables|/Script/Engine.Character|GetCapsuleComponent _player_character_2))
  (bind _returnvalue_4 (Math|Vector|GetUpVector (.rotation _returnvalue)))
  (bind _returnvalue_5 (Components|Capsule|GetScaledCapsuleHalfHeight _capsulecomponent))
  (bind _returnvalue_6 (* _returnvalue_4 -1.0))
  (bind _returnvalue_7 (* _returnvalue_6 1e+01))
  (bind _returnvalue_8 (+ (.location _returnvalue) _returnvalue_7))
  ;[0 0 0] Movement
  ;[0 0 0] Camera angle detection - Tend to leave the ladder or not
  (bind _player_character_3 (Variables|ClimbableLadder|GetPlayer%20Character)
    (:then
      (if (and (> (Variables|/Game/FirstPerson/Blueprints/BP_FirstPersonCharacter.BP_FirstPersonCharacter_C|GetMoveY (Variables|ClimbableLadder|GetPlayer%20Character)) 0.0) (Math|Float|InRange(Float) (Math|Float|Absolute(Float) (Class|KismetMathLibrary|DegAcos (Math|Vector|DotProduct (Math|Vector|MakeVector (.x (Math|Vector|GetForwardVector (Variables|/Game/FirstPerson/Blueprints/BP_FirstPersonCharacter.BP_FirstPersonCharacter_C|GetFirstPersonCamera _player_character_3))) (.y (Math|Vector|GetForwardVector (Variables|/Game/FirstPerson/Blueprints/BP_FirstPersonCharacter.BP_FirstPersonCharacter_C|GetFirstPersonCamera _player_character_3))) 0.0) (Math|Vector|GetUpVector (Variables|Default|GetSpline))))) 0.0 (Variables|ClimbableLadder|GetLeave%20Max%20Angle)))
        ;[0 0 0] Leave the ladder
        (CallFunction|ParkourLeave _player_character)
        (Character|LaunchCharacter _player_character (+ (* (Math|Vector|GetForwardVector (Variables|/Game/FirstPerson/Blueprints/BP_FirstPersonCharacter.BP_FirstPersonCharacter_C|GetFirstPersonCamera _player_character)) 5e+02) "0, 0,200.000000") true true)
        (else
          ;[0 0 0] Check if the player character can continue to move up or down
          (Variables|ClimbableLadder|SetCan%20Move%20Down (not (Math|Vector|Equal(Vector) (Spline|GetLocationatTime _spline 0.0 "World" false) (.location (Class|SplineComponent|FindTransformClosesttoWorldLocation _spline (+ _returnvalue_2 (* _returnvalue_3 (* _returnvalue_5 -1.0))) "World" false)) 1.0)))
          (Variables|ClimbableLadder|SetCan%20Move%20Up (not (Math|Vector|Equal(Vector) (Spline|GetLocationatTime _spline 1.0 "World" false) (.location (Class|SplineComponent|FindTransformClosesttoWorldLocation _spline (+ _returnvalue_2 (* _returnvalue_3 (/ _returnvalue_5 1.5))) "World" false)) 1.0)))
          ;[0 0 0] Detect player's movement inputs
          (Math|Float|CompareFloat (Variables|/Game/FirstPerson/Blueprints/BP_FirstPersonCharacter.BP_FirstPersonCharacter_C|GetMoveY (Variables|ClimbableLadder|GetPlayer%20Character)) 0.0 ; >0 to move up\n<0 to move down
            (:>
              ;[0 0 0] Can up?
              (if (Variables|ClimbableLadder|GetCan%20Move%20Up)
                ;[0 0 0] Move up or down along the spline
                (CallFunction|MoveEvent :!label _label)
                (CallFunction|ClimbShake)
                (else
                  ;[0 0 0] Top climbup trace
                  (bind _outhit (Collision|SphereTraceByChannel _returnvalue_8 (+ _returnvalue_8 (* _returnvalue_6 5e+01)) 1e+01 "TraceTypeQuery1" false (Utilities|Array|MakeArray self) (Variables|ClimbableLadder|GetDraw%20Debug))) ; Trace 1 : Forward Detection
                  (bind _output_get (Variables|ClimbableLadder|SetFwd%20Hit _outhit))
                  (if (.bBlockingHit (Collision|BreakHitResult _output_get))
                    (bind _outhit_2 (Collision|SphereTraceByChannel (+ (.Location (Collision|BreakHitResult _output_get)) (* (Math|Vector|GetForwardVector (.rotation (Spline|GetTransformatTime (Variables|Default|GetSpline) 1.0 "World" false false))) 3e+01)) (.Location (Collision|BreakHitResult _output_get)) 1e+01 "TraceTypeQuery1" false (Utilities|Array|MakeArray self) (Variables|ClimbableLadder|GetDraw%20Debug))) ; Trace 2 : Downward Detection
                    (bind _output_get_2 (Variables|ClimbableLadder|SetDwd%20Hit _outhit_2))
                    (if (and (.bBlockingHit (Collision|BreakHitResult _output_get_2)) (not (.bInitialOverlap (Collision|BreakHitResult _output_get_2))))
                      (bind _outhit_3 (Collision|SphereTraceByChannel (+ (+ (* (Class|SplineComponent|GetUpVectoratTime (Variables|Default|GetSpline) 1.0 "World" false) -4e+01) (.ImpactPoint (Collision|BreakHitResult (Variables|ClimbableLadder|GetDwd%20Hit)))) (* (.ImpactNormal (Collision|BreakHitResult (Variables|ClimbableLadder|GetDwd%20Hit))) 1.5e+02)) (+ (+ (* (Class|SplineComponent|GetUpVectoratTime (Variables|Default|GetSpline) 1.0 "World" false) -4e+01) (.ImpactPoint (Collision|BreakHitResult (Variables|ClimbableLadder|GetDwd%20Hit)))) (* (.ImpactNormal (Collision|BreakHitResult (Variables|ClimbableLadder|GetDwd%20Hit))) 4e+01)) 3e+01 "TraceTypeQuery1" false 0 (Variables|ClimbableLadder|GetDraw%20Debug))) ; Trace 3 : Climbup Space Detection
                      (if (not (.bBlockingHit (Collision|BreakHitResult _outhit_3)))
                        (CallFunction|ClimbupLedge) ; If a climbable ledge was detected,\nthen leave the ladder and climbup the ledge.
                      ))))))
            (:<
              ;[0 0 0] Can down?
              (if (Variables|ClimbableLadder|GetCan%20Move%20Down)
                (goto _label)
                (else
                  ;[0 0 0] Trace down to find if there is a walkable plane under the player character when he reaches the bottom of the ladder
                  (bind _player_character_4 (Variables|ClimbableLadder|GetPlayer%20Character)
                    (:then)
                    (:else)))))))))
    (:else)))

(event Custom|Climbup%20Ledge
  ;[0 0 0] Climb up the ledge on top
  (Utilities|Time|ClearandInvalidateTimerbyHandle (Variables|ClimbableLadder|GetMovement%20Timer)) ; Disable Movement Event
  (bind _player_character (Variables|ClimbableLadder|GetPlayer%20Character)
    (:then
      (Variables|ClimbableLadder|SetStart%20Location (Transformation|GetActorLocation _player_character)) ; Store the start position
      (Components|Timeline|PlayfromStart (Variables|Default|GetTimeline_Climbup)))
    (:else)))

(event Custom|StartClimbing
  (bind _player_character (Variables|ClimbableLadder|GetPlayer%20Character))
  ;[0 0 0] Start Enter Event
  (Collision|SetCollisionEnabled (Variables|Default|GetTop%20Collision) "NoCollision") ; Deactivate all triggers
  (Variables|/Game/FirstPerson/Blueprints/BP_FirstPersonCharacter.BP_FirstPersonCharacter_C|SetbParkour _player_character true)
  (Variables|/Game/FirstPerson/Blueprints/BP_FirstPersonCharacter.BP_FirstPersonCharacter_C|SetParkourActor _player_character self)
  (Pawn|Components|CharacterMovement|SetMovementMode (Variables|/Script/Engine.Character|GetCharacterMovement _player_character) "MOVE_Custom" 0)
  (CallFunction|EnterLadder))

(event Custom|StartLeaving
  (bind _player_character (Variables|ClimbableLadder|GetPlayer%20Character))
  ;[0 0 0] Start Leave Event
  (Collision|SetCollisionEnabled (Variables|Default|GetTop%20Collision) "QueryAndPhysics") ; Activate all triggers
  (Variables|/Game/FirstPerson/Blueprints/BP_FirstPersonCharacter.BP_FirstPersonCharacter_C|SetbParkour _player_character false)
  (Variables|/Game/FirstPerson/Blueprints/BP_FirstPersonCharacter.BP_FirstPersonCharacter_C|SetParkourActor _player_character self)
  (Pawn|Components|CharacterMovement|SetMovementMode (Variables|/Script/Engine.Character|GetCharacterMovement _player_character) "MOVE_Walking" 0)
  (Utilities|Time|ClearandInvalidateTimerbyHandle (Variables|ClimbableLadder|GetMovement%20Timer)))

(event Custom|EnterLadder
  (bind _player_character (Variables|ClimbableLadder|GetPlayer%20Character))
  (bind _spline (Variables|Default|GetSpline))
  (bind _player_character_2 (Variables|ClimbableLadder|GetPlayer%20Character))
  (bind _returnvalue (Transformation|GetActorLocation _player_character))
  (bind _capsulecomponent (Variables|/Script/Engine.Character|GetCapsuleComponent _player_character))
  (bind _returnvalue_2 (Class|SplineComponent|FindTransformClosesttoWorldLocation _spline _returnvalue "World" false))
  (bind _returnvalue_3 (Components|Capsule|GetScaledCapsuleHalfHeight _capsulecomponent))
  (bind _returnvalue_4 (Math|Vector|GetForwardVector (.rotation _returnvalue_2)))
  ;[0 0 0] Handle camera view adjustment
  (bind _player_character_3 (Variables|ClimbableLadder|GetPlayer%20Character)
    (:then
      (Variables|ClimbableLadder|SetLast%20Control%20Rotation (Pawn|GetControlRotation _player_character_3 :!class /Script/Engine.Pawn))
      (Components|Timeline|PlayfromStart (Variables|Default|GetTimeline_Camera))
      ;[0 0 0] Start ladder climbing:
      ; Snap player character to the correct position based on the spline
      (Components|MoveComponentTo (Variables|/Script/Engine.Character|GetCapsuleComponent _player_character_2) (+ (Math|Vector|SelectVector (+ (* _returnvalue_4 (* _returnvalue_3 -1.0)) (.location _returnvalue_2)) (Math|Vector|SelectVector (+ (* _returnvalue_4 (/ _returnvalue_3 1.5)) (.location _returnvalue_2)) (.location _returnvalue_2) (Math|Vector|Equal(Vector) (Spline|GetLocationatTime _spline 0.0 "World" false) (.location _returnvalue_2) _returnvalue_3)) (Math|Vector|Equal(Vector) (Spline|GetLocationatTime _spline 1.0 "World" false) (.location _returnvalue_2) (/ _returnvalue_3 1.5))) (* (Math|Vector|GetUpVector (.rotation _returnvalue_2)) (Variables|ClimbableLadder|GetDistance%20from%20front%20to%20ladder))) (Math|Rotator|Delta(Rotator) (Transformation|GetActorRotation) "0,90.000000, 0") true true 0.3 true)
      (Components|Movement|StopMovementImmediately (Variables|/Script/Engine.Character|GetCharacterMovement _player_character_2))
      ;[0 0 0] Movement Timer Setup
      (bind _returnvalue_5 (Utilities|Time|SetTimerbyEvent (EventDispatchers|CreateEvent :!event Custom|Ladder%20Movement) (Utilities|Time|GetWorldDeltaSeconds) true))
      (Variables|ClimbableLadder|SetMovement%20Timer _returnvalue_5))
    (:else)))

(event Custom|ClimbShake
  ;[0 0 0] Climb Camera Shake
  (Utilities|FlowControl|Gate false :!label _label
    (:Exit
      (Utilities|FlowControl|Sequence
        (:then_0
          (goto _label Close))
        (:then_1
          (bind _player_character (Variables|ClimbableLadder|GetPlayer%20Character)
            (:then
              (Math|Float|CompareFloat (Variables|/Game/FirstPerson/Blueprints/BP_FirstPersonCharacter.BP_FirstPersonCharacter_C|GetMoveY _player_character) 0.0
                (:>
                  _)
                (:<
                  _))
              (bind _isa (Utilities|FlowControl|FlipFlop)
                (:A
                  _)
                (:B
                  _))
              (Game|Feedback|ClientStartCameraShake (Game|GetPlayerController 0) (select _isa "/Game/FPClimbableLadder/Blueprints/CS_ClimbLadderR.CS_ClimbLadderR_C" "/Game/FPClimbableLadder/Blueprints/CS_ClimbLadderL.CS_ClimbLadderL_C") 1.0 "CameraLocal" "0, 0, 0")
              (Utilities|FlowControl|Delay 0.2)
              (goto _label Open))
            (:else)))))))

(event Custom|MoveEvent
  (bind _player_character (Variables|ClimbableLadder|GetPlayer%20Character))
  (bind _capsulecomponent (Variables|/Script/Engine.Character|GetCapsuleComponent _player_character))
  ;[0 0 0] Move up or down along the spline
  (Components|MoveComponentTo _capsulecomponent (+ (Transformation|GetWorldLocation _capsulecomponent) (* (Math|Vector|GetForwardVector (Class|SplineComponent|FindRotationClosesttoWorldLocation (Variables|Default|GetSpline) (Transformation|GetActorLocation (Variables|ClimbableLadder|GetPlayer%20Character)) "World")) (* (Variables|/Game/FirstPerson/Blueprints/BP_FirstPersonCharacter.BP_FirstPersonCharacter_C|GetMoveY (Variables|ClimbableLadder|GetPlayer%20Character)) (Variables|ClimbableLadder|GetMove%20Speed) (Utilities|Time|GetWorldDeltaSeconds)))) (Transformation|GetWorldRotation _capsulecomponent) true true (Utilities|Time|GetWorldDeltaSeconds) true))

(event EventBeginPlay
  ;[0 0 0] Begin Play : Setup for collisions
  (Collision|SetCollisionEnabled (Variables|Default|GetSide%20Collision) "QueryAndPhysics")
  (bind _aswb_input (Utilities|Casting|CastToWB_Input (UserInterface|GetUserWidgetObject (Variables|Default|GetWidget))))
  (Variables|/Game/FPClimbableLadder/Blueprints/WB_Input.WB_Input_C|SetContent _aswb_input "Interact with ladder"))

(event EventTick
  (params (DeltaSeconds :type Float%20%28single-precision%29))
  (bind _widget (Variables|Default|GetWidget))
  ;[0 0 0] Tick : Move the widget along Spline with smooth transition when it's visible to ensure that Player can understand which input key can be clicked to climb up the ladder.
  (if (Rendering|IsVisible (Variables|Default|GetWidget))
    (bind _player_character (Variables|ClimbableLadder|GetPlayer%20Character)
      (:then
        (Transformation|SetWorldLocation _widget (Math|Interpolation|VInterpTo (Transformation|GetWorldLocation _widget) (+ (.location (Class|SplineComponent|FindTransformClosesttoWorldLocation (Variables|Default|GetSpline) (Transformation|GetWorldLocation (Variables|/Game/FirstPerson/Blueprints/BP_FirstPersonCharacter.BP_FirstPersonCharacter_C|GetFirstPersonCamera _player_character)) "World" false)) (* (Math|Vector|GetUpVector (.rotation (Class|SplineComponent|FindTransformClosesttoWorldLocation (Variables|Default|GetSpline) (Transformation|GetWorldLocation (Variables|/Game/FirstPerson/Blueprints/BP_FirstPersonCharacter.BP_FirstPersonCharacter_C|GetFirstPersonCamera _player_character)) "World" false))) 1e+01)) (Utilities|Time|GetWorldDeltaSeconds) 3e+01) false false))
      (:else))))

(event EventParkourEnter
  (params (Character :type Character%20Object%20Reference))
  (bind _spline (Variables|Default|GetSpline))
  (bind _player_character (Variables|ClimbableLadder|GetPlayer%20Character))
  (bind _returnvalue (Pawn|GetControlRotation _player_character :!class /Script/Engine.Pawn))
  (bind _firstpersoncamera (Variables|/Game/FirstPerson/Blueprints/BP_FirstPersonCharacter.BP_FirstPersonCharacter_C|GetFirstPersonCamera _player_character))
  (bind _returnvalue_2 (Transformation|GetWorldLocation _firstpersoncamera))
  (bind _returnvalue_3 (Math|Vector|GetForwardVector _returnvalue))
  (bind _returnvalue_4 (Spline|FindLocationClosesttoWorldLocation _spline _returnvalue_2 "World"))
  (bind _returnvalue_5 (- _returnvalue_4 _returnvalue_2))
  (bind _returnvalue_6 (Math|Vector|Normalize _returnvalue_5))
  (bind _returnvalue_7 (Math|Vector|DotProduct _returnvalue_6 _returnvalue_3))
  (bind _returnvalue_8 (Class|KismetMathLibrary|DegAcos _returnvalue_7))
  (bind _returnvalue_9 (Math|Float|Absolute(Float) _returnvalue_8))
  ;[0 0 0] BPI Parkour Enter
  (Utilities|IsValid Character
    (:Is%20Valid
      (if (== Character (Variables|ClimbableLadder|GetPlayer%20Character))
        ;[0 0 0] Is pawn in trigger
        (if (Collision|IsOverlappingActor (Variables|Default|GetSide%20Collision) (Variables|ClimbableLadder|GetPlayer%20Character) :!class /Script/Engine.PrimitiveComponent)
          ;[0 0 0] Detection for enter look angle
          (if (Math|Float|InRange(Float) _returnvalue_9 0.0 (Variables|ClimbableLadder|GetEnter%20Max%20Angle%20Side))
            ;[0 0 0] Call start climbing event
            (CallFunction|StartClimbing :!label _label))
          (elif (Collision|IsOverlappingActor (Variables|Default|GetTop%20Collision) (Variables|ClimbableLadder|GetPlayer%20Character) :!class /Script/Engine.PrimitiveComponent)
            (if (Math|Float|InRange(Float) _returnvalue_9 0.0 (Variables|ClimbableLadder|GetEnter%20Max%20Angle%20Top))
              (goto _label))))))))

(event EventParkourLeave
  (params (Character :type Character%20Object%20Reference))
  ;[0 0 0] BPI Parkour Leave
  (Utilities|IsValid Character
    (:Is%20Valid
      (if (== Character (Variables|ClimbableLadder|GetPlayer%20Character))
        ;[0 0 0] Call start leaving event
        (CallFunction|StartLeaving)))))

(fn ConstructionScript
  (bind _returnvalue (Math|Float|MakeLiteralFloat 2e+01))
  (bind _top_collision (Variables|Default|GetTop%20Collision))
  (bind _spline (Variables|Default|GetSpline))
  (bind _side_collision (Variables|Default|GetSide%20Collision))
  (Utilities|FlowControl|Sequence
    (:then_0
      ;[0 0 0] Spawn the ladder
      (for _index (range 0 (- (Variables|ClimbableLadder|GetLadder%20Height) 1))
        (AddComponent|AddStaticMeshComponent false (Math|Transform|MakeTransform (* "0, 0,60.000000" _index) "0, 0, 0" "1.000000,1.000000,1.000000"))))
    (:then_1
      ;[0 0 0] Spline points setup
      (Spline|SetLocationatSplinePoint _spline (- (Spline|GetNumberOfSplinePoints _spline) 1) (* "60.000000, 0,0.000000" (Variables|ClimbableLadder|GetLadder%20Height)) "Local" true))
    (:then_2
      ;[0 0 0] Side Collision Setup
      (Transformation|SetRelativeLocation _side_collision (Math|Vector|MakeVector 0.0 (/ (Variables|ClimbableLadder|GetEnter%20Extent) 2.0) (/ (* (Variables|ClimbableLadder|GetLadder%20Height) 6e+01) 2.0)) false false)
      (Components|Box|SetBoxExtent _side_collision (Math|Vector|MakeVector 3e+01 (/ (Variables|ClimbableLadder|GetEnter%20Extent) 2.0) (* (Variables|ClimbableLadder|GetLadder%20Height) 3e+01)) true))
    (:then_3
      ;[0 0 0] Top Collision Setup
      (Transformation|SetRelativeLocation _top_collision (Math|Vector|MakeVector 0.0 (* (/ (Variables|ClimbableLadder|GetEnter%20Extent) 2.0) -1.0) (+ (* (Variables|ClimbableLadder|GetLadder%20Height) 6e+01) _returnvalue)) false false)
      (Components|Box|SetBoxExtent _top_collision (Math|Vector|MakeVector 3e+01 (/ (Variables|ClimbableLadder|GetEnter%20Extent) 2.0) _returnvalue) true))))