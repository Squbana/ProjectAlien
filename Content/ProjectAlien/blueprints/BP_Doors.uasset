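; BP_Doors is an automatic double sliding door that opens when the first-person character enters its Box trigger and closes when that character leaves.
; Two timelines, LeftDoorAnimation and RightDoorAnimation, drive the relative X location of Door1 and Door2.
; Overlap begin plays both timelines, while overlap end reverses them from the end, so closing always starts from the fully open position.
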(event OnComponentBeginOverlap(Box)
  (params (OverlappedComponent :type Primitive%20Component%20Object%20Reference) (OtherActor :type Actor%20Object%20Reference) (OtherComp :type Primitive%20Component%20Object%20Reference) (OtherBodyIndex :type Integer) (bFromSweep :type Boolean) (SweepResult :type Hit%20Result%20Structure%20%28by%20ref%29))
  ;[1 1 1] Opening doors
  (Utilities|Casting|CastToBP_FirstPersonCharacter OtherActor)
  (Utilities|FlowControl|Sequence
    (:then_0
      (bind _leftdoorvalue (Timeline|LeftDoorAnimation Play)
        (:Update
          (Transformation|SetRelativeLocation (Variables|Default|Getdoor1) (Math|Vector|MakeVector _leftdoorvalue 0.0 0.0) false false))))
    (:then_1
      (bind _right_door_value (Timeline|RightDoorAnimation Play)
        (:Update
          (Transformation|SetRelativeLocation (Variables|Default|Getdoor2) (Math|Vector|MakeVector _right_door_value 0.0 0.0) false false))))))

(event OnComponentEndOverlap(Box)
  (params (OverlappedComponent :type Primitive%20Component%20Object%20Reference) (OtherActor :type Actor%20Object%20Reference) (OtherComp :type Primitive%20Component%20Object%20Reference) (OtherBodyIndex :type Integer))
  ;[1 1 1] Closing Doors
  (Utilities|Casting|CastToBP_FirstPersonCharacter OtherActor)
  (Utilities|FlowControl|Sequence
    (:then_0
      (bind _leftdoorvalue (Timeline|LeftDoorAnimation ReverseFromEnd)
        (:Update
          (Transformation|SetRelativeLocation (Variables|Default|Getdoor1) (Math|Vector|MakeVector _leftdoorvalue 0.0 0.0) false false))))
    (:then_1
      (bind _right_door_value (Timeline|RightDoorAnimation ReverseFromEnd)
        (:Update
          (Transformation|SetRelativeLocation (Variables|Default|Getdoor2) (Math|Vector|MakeVector _right_door_value 0.0 0.0) false false))))))

(fn ConstructionScript)