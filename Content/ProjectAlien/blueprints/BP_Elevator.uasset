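; BP_Elevator is an elevator actor that moves vertically by a set Distance.
; The ElevatorMove custom event derives FinalLocation from StartLocation plus Distance, then plays the Elevated timeline.
; Each timeline update lerps the actor's Z between the two heights using the Elevating track, keeping X and Y unchanged.
; StartLocation is only assigned to itself, and nothing in this Blueprint calls ElevatorMove.
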(event Custom|ElevatorMove
  (bind _returnvalue (Transformation|GetActorLocation))
  ;[1 1 1] Elevating
  (bind _output_get (Variables|Default|SetStartLocation (Variables|Default|GetStartLocation)))
  (Variables|Default|SetFinalLocation (+ _output_get (Variables|Default|GetDistance)))
  (bind _elevating (Timeline|Elevated Play)
    (:Update
      (Transformation|SetActorLocation (Math|Vector|MakeVector (.x _returnvalue) (.y _returnvalue) (Math|Float|Lerp (Variables|Default|GetStartLocation) (Variables|Default|GetFinalLocation) _elevating)) false false))))

(fn ConstructionScript)